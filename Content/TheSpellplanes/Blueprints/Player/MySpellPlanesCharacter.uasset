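; Player character Blueprint for Spellplanes that handles gear visuals and hit reactions, and moves to a fixed location on BeginPlay.
; Gear changes look up the slot in PlayerMeshes but always set ChestMesh, with debug prints around an unresolved map issue.
; Point damage plays a random hit-react montage and spawns test particles at the impact.
; The construction script adds the character to its SceneCapture's show-only list.
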(event Custom|PlayHitFX
  (params (Damage :type Float%20%28single-precision%29) (DamageType :type Damage%20Type%20Object%20Reference) (Hit :type Hit%20Result%20Structure) (PointDamage :type Boolean))
  (bind (_bblockinghit _binitialoverlap _time _distance _location _impactpoint _normal _impactnormal) (Collision|BreakHitResult Hit))
  (bind _hitreactanimations (Variables|FX|GetHitReactAnimations))
  (bind _returnvalue (Utilities|Array|Length _hitreactanimations))
  (bind _returnvalue_2 (- _returnvalue 1))
  (bind _returnvalue_3 (Math|Random|RandomIntegerinRange 0 _returnvalue_2))
  (bind _output (Utilities|Array|Get(acopy) _hitreactanimations _returnvalue_3))
  (Utilities|IsValid _output
    (:Is%20Valid
      (Animation|PlayAnimMontage _output 1.0 "None"))
    (:Is%20Not%20Valid
      _))
  (if PointDamage
    (Effects|SpawnEmitteratLocation "/Game/TheSpellplanes/Assets/Particles/TestParticles.TestParticles" _location (Math|Conversions|RotationFromXVector _impactnormal))))

(event Custom|OnEquippedGearChanged_Event_0
  (params (Slot :type EEquippableSlot%20Enum :default "EIS_Head") (Gear :type Gear%20Item%20Object%20Reference))
  ;[1 1 1] THIS PROVES that the issue is in the PlayerMesh TMap and how it is storing the component.
  (Development|PrintString "Hello")
  (if (.ReturnValue (Utilities|Map|Find (Variables|Default|GetPlayerMeshes) Slot))
    (Class|SkinnedMeshComponent|SetSkeletalMesh (Variables|Default|GetChestMesh) (Variables|/Script/TheSpellplanes.GearItem|GetMesh Gear) false)
    (else
      (Development|PrintString "CANT FINDS MESH COMPONENT" true true "(R=1.000000,G=0.009362,B=0.000000,A=1.000000)" 1e+01))))

(event EventBeginPlay
  (EventDispatchers|AssignOnEquippedGearChanged (delegate Custom|OnEquippedGearChanged_Event_0))
  (Transformation|SetActorLocation "200.000000,200.000000,19.000000" false false))

(event Game|Damage|EventPointDamage
  (params (Damage :type Float%20%28single-precision%29) (DamageType :type Damage%20Type%20Object%20Reference) (HitLocation :type Vector :default "0, 0, 0") (HitNormal :type Vector :default "0, 0, 0") (HitComponent :type Primitive%20Component%20Object%20Reference) (BoneName :type Name :default "None") (ShotFromDirection :type Vector :default "0, 0, 0") (InstigatedBy :type Controller%20Object%20Reference) (DamageCauser :type Actor%20Object%20Reference) (HitInfo :type Hit%20Result%20Structure%20%28by%20ref%29))
  (CallFunction|PlayHitFX Damage DamageType HitInfo true))

(fn ConstructionScript
  (Utilities|Array|AddUnique (Variables|/Script/Engine.SceneCaptureComponent|GetShowOnlyActors (Variables|Default|GetSceneCaptureComponent2D)) self))
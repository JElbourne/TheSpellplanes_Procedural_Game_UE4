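; Player controller for Spellplanes that owns the player's UI: inventory, pause menu, in-game UI, notifications, death screen and loot menu.
; Most widgets are created lazily and cached, while the loot menu is rebuilt on each show.
; Inventory switches to UI-only input, pausing halts the game, and the in-game UI and death screen clear all widgets first.
; Notifications feed a stack widget, with a B-key test message left in.
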(event Custom|CreateNotificationUI
  (Utilities|IsValid (Variables|Default|GetWBP_NotificationWidget)
    (:Is%20Valid
      _)
    (:Is%20Not%20Valid
      (bind _returnvalue (UserInterface|CreateWidget "/Game/TheSpellplanes/UserInterface/Widgets/WBP_NotificationStack.WBP_NotificationStack_C"))
      (Variables|Default|SetWBP_NotificationWidget _returnvalue)))
  (UserInterface|Viewport|AddtoViewport (Variables|Default|GetWBP_NotificationWidget) 0))

(event Custom|AddInGameUI
  (Utilities|IsValid (Variables|Default|GetWBP_GameUI)
    (:Is%20Valid
      _)
    (:Is%20Not%20Valid
      (bind _returnvalue (UserInterface|CreateWidget "/Game/TheSpellplanes/UserInterface/Widgets/WBP_GameUI.WBP_GameUI_C"))
      (Variables|Default|SetWBP_GameUI _returnvalue)))
  (UserInterface|Viewport|AddtoViewport (Variables|Default|GetWBP_GameUI) 0))

(event Custom|OpenPauseMenu
  (Utilities|IsValid (Variables|Default|GetWBP_PauseMenu)
    (:Is%20Valid
      _)
    (:Is%20Not%20Valid
      (bind _returnvalue (UserInterface|CreateWidget "/Game/TheSpellplanes/UserInterface/Widgets/WBP_PauseMenu.WBP_PauseMenu_C"))
      (Variables|Default|SetWBP_PauseMenu _returnvalue)))
  (UserInterface|Viewport|AddtoViewport (Variables|Default|GetWBP_PauseMenu) 0)
  (Game|SetGamePaused true))

(event Custom|ClosePauseMenu
  (bind _wbp_pausemenu (Variables|Default|GetWBP_PauseMenu))
  (Utilities|IsValid _wbp_pausemenu
    (:Is%20Valid
      (Widget|RemovefromParent _wbp_pausemenu)
      (Game|SetGamePaused false))))

(event EventShowIngameUI
  (if (Pawn|IsLocalPlayerController)
    (Viewport|RemoveAllWidgets)
    (CallFunction|AddinGameUI)
    (CallFunction|CreateNotificationUI)))

(event EventShowNotification
  (params (Message :type Text%20%28by%20ref%29))
  (bind _wbp_notificationwidget (Variables|Default|GetWBP_NotificationWidget))
  (Utilities|IsValid _wbp_notificationwidget
    (:Is%20Valid
      (Default|AddNotification _wbp_notificationwidget Message))))

(event EventShowLootMenu
  (params (LootSource :type Inventory%20Component%20Object%20Reference))
  (bind _returnvalue (UserInterface|CreateWidget "/Game/TheSpellplanes/UserInterface/Widgets/WBP_LootMenu.WBP_LootMenu_C"))
  (bind _output_get (Variables|Default|SetWBP_LootMenu _returnvalue))
  (UserInterface|Viewport|AddtoViewport _output_get 0))

(event EventHideLootMenu
  (Widget|RemovefromParent (Variables|Default|GetWBP_LootMenu)))

(event EventBeginPlay
  (Utilities|IsValid (Variables|Default|GetWBP_InventoryWidget)
    (:Is%20Not%20Valid
      (bind _returnvalue (UserInterface|CreateWidget "/Game/TheSpellplanes/UserInterface/Widgets/WBP_Inventory.WBP_Inventory_C"))
      (Variables|Default|SetWBP_InventoryWidget _returnvalue))))

(event EventShowDeathScreen
  (params (Killer :type Spell%20Planes%20Character%20Object%20Reference))
  (Viewport|RemoveAllWidgets)
  (Utilities|IsValid (Variables|Default|GetWBP_DeathScreen)
    (:Is%20Valid
      _)
    (:Is%20Not%20Valid
      (bind _returnvalue (UserInterface|CreateWidget "/Game/TheSpellplanes/UserInterface/Widgets/WBP_DeathScreen.WBP_DeathScreen_C" 0 Killer))
      (Variables|Default|SetWBP_DeathScreen _returnvalue)))
  (UserInterface|Viewport|AddtoViewport (Variables|Default|GetWBP_DeathScreen) 0))

(event Input|ActionEvents|InputActionOpenInventory
  (params (Key :type Key%20Structure :default "None"))
  (:Pressed
    (Utilities|IsValid (Variables|Default|GetWBP_InventoryWidget)
      (:Is%20Valid
        _)
      (:Is%20Not%20Valid
        (bind _returnvalue (UserInterface|CreateWidget "/Game/TheSpellplanes/UserInterface/Widgets/WBP_Inventory.WBP_Inventory_C"))
        (Variables|Default|SetWBP_InventoryWidget _returnvalue)))
    (UserInterface|Viewport|AddtoViewport (Variables|Default|GetWBP_InventoryWidget) 0)
    (Variables|Default|SetbShowMouseCursor true)
    (Input|SetInputModeUIOnly self 0 "DoNotLock")))

(event Input|ActionEvents|InputActionPauseMenu
  (params (Key :type Key%20Structure :default "None"))
  (:Pressed
    (CallFunction|OpenPauseMenu)
    (Development|PrintString "LETS PAUSE")))

(event Input|KeyboardEvents|B
  (params (Key :type Key%20Structure :default "None"))
  (:Pressed
    (Class|SpellPlanesPlayerController|ClientShowNotification (Utilities|Text|MakeLiteralText "Hello This is a notification."))))

(fn ConstructionScript)
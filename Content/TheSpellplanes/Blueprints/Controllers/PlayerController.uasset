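; Player controller for a block-based game, whose only live logic caches BP_GameInstance in the construction script; BeginPlay and Tick are empty.
; Disconnected graphs hold logic to spawn a grid highlighter and HUD widget.
; Other unwired chains trace under the mouse by placing or attacking mode, highlighting blocks the character overlaps.
; An unwired action chain uses the active action-bar item or damages IAttackable blocks.
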(event EventTick
  (params (DeltaSeconds :type Float%20%28single-precision%29)))

(event EventBeginPlay)

(event Input|ActionEvents|InputActionUse
  (params (Key :type Key%20Structure :default "None")))

(fn ConstructionScript
  (bind _asbp_game_instance (Utilities|Casting|CastToBP_GameInstance (Game|GetGameInstance)))
  (Variables|Default|SetGameINstance _asbp_game_instance))
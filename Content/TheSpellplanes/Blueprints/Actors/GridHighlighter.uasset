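; GridHighlighter is an actor that shows or hides a highlight cube, likely to mark a cell on a grid.
; The construction script creates a dynamic material instance of Mat_GridHighlight on the cube and stores it as HighlightMaterial.
; ShowHighlighter and HideHighlighter toggle the cube's visibility after a validity check, and the event graph holds no active logic.
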(event EventBeginPlay)

(event Collision|EventActorBeginOverlap
  (params (OtherActor :type Actor%20Object%20Reference)))

(event EventTick
  (params (DeltaSeconds :type Float%20%28single-precision%29)))

(fn ConstructionScript
  (bind _returnvalue (Rendering|Material|CreateDynamicMaterialInstance (Variables|Default|GetHighlightCube) 0 "/Game/TheSpellplanes/Materials/Mat_GridHighlight.Mat_GridHighlight" "None" :!class /Script/Engine.PrimitiveComponent))
  (Variables|Default|SetHighlightMaterial _returnvalue))

(fn ShowHighlighter
  (bind _highlightcube (Variables|Default|GetHighlightCube))
  (Utilities|IsValid _highlightcube
    (:Is%20Valid
      (Rendering|SetVisibility _highlightcube true false))))

(fn HideHighlighter
  (bind _highlightcube (Variables|Default|GetHighlightCube))
  (Utilities|IsValid _highlightcube
    (:Is%20Valid
      (Rendering|SetVisibility _highlightcube false false))))
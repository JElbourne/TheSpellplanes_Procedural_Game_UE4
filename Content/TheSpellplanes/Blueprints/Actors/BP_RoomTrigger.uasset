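; BP_RoomTrigger is a trigger actor that sets off movement between rooms when the player walks into it.
; A player overlap on LevelTrigger passes the actor's location to BP_GameInstance to spawn the next areas.
; On BeginPlay it binds to the game instance's new-room event, which runs custom culling with destroy enabled, using its room location and the new room center.
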(event OnComponentBeginOverlap(LevelTrigger)
  (params (OverlappedComponent :type Primitive%20Component%20Object%20Reference) (OtherActor :type Actor%20Object%20Reference) (OtherComp :type Primitive%20Component%20Object%20Reference) (OtherBodyIndex :type Integer) (bFromSweep :type Boolean) (SweepResult :type Hit%20Result%20Structure%20%28by%20ref%29))
  (bind _returnvalue (Game|GetPlayerCharacter 0))
  ;[1 1 1] Trigger that will set off the movement between rooms
  (if (== OtherActor _returnvalue)
    (bind _asbp_game_instance (Utilities|Casting|CastToBP_GameInstance (Game|GetGameInstance)))
    (Default|CallSpawnNextAreas _asbp_game_instance (Transformation|GetActorLocation))
    (Utilities|Casting|CastToMySpellPlanesCharacter _returnvalue)))

(event Custom|BeginBlockCulling
  (params (NewRoomCenterWorldLocation :type Vector))
  ;[1 1 1] BIND the event to custom cull this Actor
  (Default|CustomCulling (stale EventBeginPlay _asbp_game_instance) (Variables|Transformation|GetRootComponent) (Transformation|GetActorLocation) NewRoomCenterWorldLocation (Variables|Default|GetRoomLocation) true))

(event EventBeginPlay
  ;[1 1 1] BIND the event to custom cull this Actor
  (bind _asbp_game_instance (Utilities|Casting|CastToBP_GameInstance (Game|GetGameInstance)))
  (EventDispatchers|BindEventtoWalkedIntoNewRoom _asbp_game_instance (delegate Custom|BeginBlockCulling)))

(fn ConstructionScript)
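; PathMarker is a world actor that sends the player back to the MainMenu level when their character overlaps its sphere.
; On overlap it has the game instance reset the spawned-room array and the level's block data before opening that level.
; It also binds to the game instance's walked-into-new-room event, passing its location and room location to custom culling with actor destruction enabled.
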(event OnComponentBeginOverlap(Sphere1)
  (params (OverlappedComponent :type Primitive%20Component%20Object%20Reference) (OtherActor :type Actor%20Object%20Reference) (OtherComp :type Primitive%20Component%20Object%20Reference) (OtherBodyIndex :type Integer) (bFromSweep :type Boolean) (SweepResult :type Hit%20Result%20Structure%20%28by%20ref%29))
  (Utilities|Casting|CastToMySpellPlanesCharacter OtherActor)
  (bind _asbp_game_instance (Utilities|Casting|CastToBP_GameInstance (Game|GetGameInstance)))
  (Default|ResetSpawnedRoomArray _asbp_game_instance)
  (Default|ResetBlocksinLevelData _asbp_game_instance)
  (Game|OpenLevel(byName) "MainMenu"))

(event Custom|BeginBlockCulling
  (params (NewRoomCenterWorldLocation :type Vector))
  (Default|CustomCulling (stale EventBeginPlay _asbp_game_instance) (Variables|Transformation|GetRootComponent) (Transformation|GetActorLocation) NewRoomCenterWorldLocation (Variables|Default|GetRoomLocation) true))

(event EventBeginPlay
  (bind _asbp_game_instance (Utilities|Casting|CastToBP_GameInstance (Game|GetGameInstance)))
  (EventDispatchers|BindEventtoWalkedIntoNewRoom _asbp_game_instance (delegate Custom|BeginBlockCulling)))

(fn ConstructionScript)
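; Procedural level generator actor that builds a grid of block-based rooms and places the player portal and final-room marker.
; CreateSolutionPath random-walks sideways and upward without backtracking, fixing room types so exits connect and recording start, middle and final rooms.
; SpawnArea draws the four unspawned neighbours of a location, reusing saved blocks or picking random DataTable templates by room type.
; BP_GameInstance stores level data and handles camera-distance culling.
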(event Custom|SpawnNextArea
  (params (CurrentRoomCenterWorldLocation :type Vector))
  (Variables|LocalLevelData|SetCurrentRoomWorldLocation CurrentRoomCenterWorldLocation))

(event EventBeginPlay)

(fn ConstructionScript)

(fn DrawRoom
  (params (RoomCenterWorldLocation :type Vector) (_CurrentCameraLocation :type Vector))
  (bind _spellplanesinstance (Variables|Default|GetSpellplanesInstance))
  (bind _spellplanesinstance_2 (Variables|Default|GetSpellplanesInstance))
  (bind _roomsizeinblocks (Variables|/Game/TheSpellplanes/Blueprints/BP_GameInstance.BP_GameInstance_C|GetRoomSizeInBlocks _spellplanesinstance))
  (bind _blocksize (Variables|/Game/TheSpellplanes/Blueprints/BP_GameInstance.BP_GameInstance_C|GetBlockSize _spellplanesinstance_2))
  (Utilities|FlowControl|Sequence
    (:then_0
      (LocalVariables|SetRoomCenterLocation RoomCenterWorldLocation))
    (:then_1
      (LocalVariables|SetCameraLocation _CurrentCameraLocation))
    (:then_2
      (bind _startingworldlocation (Utilities|DetermineStartingVector (Variables|Default|GetSpellplanesInstance) (LocalVariables|GetRoomCenterLocation))
        (:out
          (LocalVariables|SetStartWorldLocation _startingworldlocation)
          (Default|SetRoomTypeforLevelData (Variables|Default|GetSpellplanesInstance) (LocalVariables|GetRoomCenterLocation) (Variables|LocalLevelData|GetCurrentRoomtype))
          (LocalVariables|SetindexX 0)
          (for _index (range 0 (- (* _roomsizeinblocks _roomsizeinblocks) 1))
            ;[1 1 1] Determines location in 2D space from index while looping through Array
            (LocalVariables|SetindexX (.ReturnValue (Math|Float|Division(WholeandRemainder) (Math|Conversions|ToFloat(Integer) _index) (Math|Conversions|ToFloat(Integer) _roomsizeinblocks))))
            (LocalVariables|SetindexY (Math|Float|Truncate (.Remainder (Math|Float|Division(WholeandRemainder) (Math|Conversions|ToFloat(Integer) _index) (Math|Conversions|ToFloat(Integer) _roomsizeinblocks)))))
            ;[1 1 1] Looks for Block in Saved Data
            (bind (_block _found) (Default|GetBlockinLevelData (Variables|Default|GetSpellplanesInstance) (Math|Vector|MakeVector (- (.X (Math|Vector|BreakVector (LocalVariables|GetStartWorldLocation))) (Math|Conversions|ToFloat(Integer) (* (LocalVariables|GetindexX) _blocksize))) (+ (.Y (Math|Vector|BreakVector (LocalVariables|GetStartWorldLocation))) (Math|Conversions|ToFloat(Integer) (* (LocalVariables|GetindexY) _blocksize))) 0.0)))
            ;[1 1 1] Is location saved in Room Data
            (if _found
              ;[1 1 1] Set Type of Block from Saved Data
              (if (Utilities|IsValidClass _block)
                (LocalVariables|SetCurrentBlockType _block)
                ;[1 1 1] Spawn the Block
                (Default|SetBlockinLevelData (Variables|Default|GetSpellplanesInstance) (Math|Vector|MakeVector (- (.X (Math|Vector|BreakVector (LocalVariables|GetStartWorldLocation))) (Math|Conversions|ToFloat(Integer) (* (LocalVariables|GetindexX) _blocksize))) (+ (.Y (Math|Vector|BreakVector (LocalVariables|GetStartWorldLocation))) (Math|Conversions|ToFloat(Integer) (* (LocalVariables|GetindexY) _blocksize))) 0.0) (LocalVariables|GetCurrentBlockType) :!label _label)
                (bind _returnvalue (Game|SpawnActorfromClass (LocalVariables|GetCurrentBlockType) (Math|Conversions|ToTransform(Vector) (Math|Vector|MakeVector (- (.X (Math|Vector|BreakVector (LocalVariables|GetStartWorldLocation))) (Math|Conversions|ToFloat(Integer) (* (LocalVariables|GetindexX) _blocksize))) (+ (.Y (Math|Vector|BreakVector (LocalVariables|GetStartWorldLocation))) (Math|Conversions|ToFloat(Integer) (* (LocalVariables|GetindexY) _blocksize))) 0.0)) "AlwaysSpawn" 0 0))
                (Variables|/Game/TheSpellplanes/Blueprints/Actors/Blocks/BP_BasePhysicalBlock.BP_BasePhysicalBlock_C|SetRoomLocation _returnvalue (LocalVariables|GetRoomCenterLocation))
                ;[1 1 1] Check to see if new block is close to camera, if not Hide it.
                (if (!= (LocalVariables|GetCurrentBlockType) "/Game/TheSpellplanes/Blueprints/Actors/Blocks/BP_GridBlock.BP_GridBlock_C")
                  (Default|CustomCulling (Variables|Default|GetSpellplanesInstance) (Variables|/Script/Engine.Actor|GetRootComponent _returnvalue) (Transformation|GetActorLocation _returnvalue) (LocalVariables|GetCameraLocation) (LocalVariables|GetRoomCenterLocation) false)))
              (else
                ;[1 1 1] Determines a rendom Room Template based on a Room Type. Only used if Block not found in Room Data.
                (bind _returnvalue_2 (Utilities|GetDataTableRow "/Game/TheSpellplanes/Data/RoomTemplatesOLD.RoomTemplatesOLD" (Utilities|String|StringToName (Utilities|String|EnumtoString (Variables|LocalLevelData|GetCurrentRoomtype))))
                  (:then
                    (LocalVariables|SetRoomTemplate (Utilities|Struct|BreakST_RoomTemplate (Utilities|Array|Get(acopy) (Utilities|Struct|BreakST_RoomTemplateVariations _returnvalue_2) (Math|Random|RandomInteger (Utilities|Array|Length (Utilities|Struct|BreakST_RoomTemplateVariations _returnvalue_2))))))
                    ;[1 1 1] Set Type Of Block from Room Template
                    (LocalVariables|SetCurrentBlockType (Utilities|Array|Get(acopy) (Variables|LevelAssets|GetBlocks) (Utilities|Array|Get(acopy) (LocalVariables|GetRoomTemplate) _index)))
                    (goto _label)))))))))
    (:then_3
      (bind _returnvalue_3 (Game|SpawnActorfromClass "/Game/TheSpellplanes/Blueprints/Actors/Floors/BP_GeneralFloor.BP_GeneralFloor_C" (Math|Conversions|ToTransform(Vector) (LocalVariables|GetRoomCenterLocation)) "Undefined" 0 0))
      (Variables|/Game/TheSpellplanes/Blueprints/Actors/Floors/BP_BaseFloor.BP_BaseFloor_C|SetRoomLocation _returnvalue_3 (LocalVariables|GetRoomCenterLocation))
      (Default|CustomCulling (Variables|Default|GetSpellplanesInstance) (Variables|/Script/Engine.Actor|GetRootComponent _returnvalue_3) (Transformation|GetActorLocation _returnvalue_3) (LocalVariables|GetCameraLocation) (LocalVariables|GetRoomCenterLocation) false))
    (:then_4
      (bind _returnvalue_4 (Game|SpawnActorfromClass "/Game/TheSpellplanes/Blueprints/Actors/BP_RoomTrigger.BP_RoomTrigger_C" (Math|Conversions|ToTransform(Vector) (LocalVariables|GetRoomCenterLocation)) "Undefined" 0 0))
      (Variables|/Game/TheSpellplanes/Blueprints/Actors/BP_RoomTrigger.BP_RoomTrigger_C|SetRoomLocation _returnvalue_4 (LocalVariables|GetRoomCenterLocation))
      (Default|CustomCulling (Variables|Default|GetSpellplanesInstance) (Variables|/Script/Engine.Actor|GetRootComponent _returnvalue_4) (Transformation|GetActorLocation _returnvalue_4) (LocalVariables|GetCameraLocation) (LocalVariables|GetRoomCenterLocation) false))))

(fn SpawnArea
  (params (_CameraWorldLocation :type Vector) (RoomWorldSize :type Integer))
  (LocalVariables|SetRoomSize (Math|Conversions|ToFloat(Integer) RoomWorldSize))
  (LocalVariables|SetCameraWorldLocation _CameraWorldLocation)
  (Utilities|FlowControl|Sequence
    (:then_0
      ;[1 1 1] Grid -1,0
      (Utilities|SpawnNextRoom (* (LocalVariables|GetRoomSize) -1.0) (LocalVariables|GetCameraWorldLocation) (* (LocalVariables|GetRoomSize) 0.0)))
    (:then_1
      ;[1 1 1] Grid 0,1
      (Utilities|SpawnNextRoom (* (LocalVariables|GetRoomSize) 0.0) (LocalVariables|GetCameraWorldLocation) (* (LocalVariables|GetRoomSize) 1.0)))
    (:then_2
      ;[1 1 1] Grid 1,0
      (Utilities|SpawnNextRoom (* (LocalVariables|GetRoomSize) 1.0) (LocalVariables|GetCameraWorldLocation) (* (LocalVariables|GetRoomSize) 0.0)))
    (:then_3
      ;[1 1 1] Grid 0, -1
      (Utilities|SpawnNextRoom (* (LocalVariables|GetRoomSize) 0.0) (LocalVariables|GetCameraWorldLocation) (* (LocalVariables|GetRoomSize) -1.0)))
    (:then_4
      ;[1 1 1] Remove distant rooms from Spawned Array
      (Default|CleanSpawnedRoomArray (Variables|Default|GetSpellplanesInstance) "0, 0, 0"))))

(fn CreateSolutionPath
  (bind _returnvalue (Class|KismetSystemLibrary|MakeLiteralInteger 1))
  (bind _returnvalue_2 (Class|KismetSystemLibrary|MakeLiteralInteger 2))
  (bind _returnvalue_3 (Class|KismetSystemLibrary|MakeLiteralInteger 5))
  (bind _pathmap (LocalVariables|GetPathMap))
  (bind _array (Utilities|Array|MakeArray _returnvalue _returnvalue_2 _returnvalue_3))
  (Utilities|FlowControl|Sequence
    (:then_0
      (LocalVariables|SetupCounter 0)
      (Development|PrintString "Creating New Solution Path" true true "(R=0.000000,G=0.660000,B=1.000000,A=1.000000)" 1e+01))
    (:then_1
      (LocalVariables|SetLastRow false))
    (:then_2
      (LocalVariables|SetisGenerating true)
      ;[1 1 1] Picks a random Start Room on the first row (x)
      (bind _output_get (LocalVariables|SetCurrentPosition (Utilities|Struct|MakeIntVector 0 0)))
      (bind _output_get_2 (LocalVariables|SetStartRoom _output_get))
      (Utilities|Map|Add (LocalVariables|GetPathMap) _output_get_2 (Utilities|Enum|LiteralenumRoomTypes (Utilities|Enum|ByteToEnumRoomTypes (Math|Conversions|ToByte(Integer) (Math|Random|RandomIntegerinRange 0 1)))))
      ;[1 1 1] Set Intial Direction
      (LocalVariables|SetDirection (Math|Random|RandomIntegerinRange 1 5))
      ;[1 1 1] Begin Loop
      (while (LocalVariables|GetisGenerating)
        ;[0.2764 0.9202 1 1 50] Loop Body
        (switch int (LocalVariables|GetDirection)
          (:1
            ;;[1 1 1] Move Right
            (bind _result (Math|Integer|IncrementInt (Utilities|Struct|BreakIntVector (LocalVariables|GetCurrentPosition)) :!label _label)
              (:%20%20
                (Utilities|Struct|SetmembersinIntVector (LocalVariables|GetCurrentPosition) _result)
                ;;[1 1 1] Next Direction, Can not backtrack
                (LocalVariables|SetDirection (Utilities|Array|Get(acopy) _array (Math|Random|RandomInteger (Utilities|Array|Length _array))))
                ;;[1 1 1] Add Any Type of Room
                (LocalVariables|SetSelectedRoomType (Utilities|GetRandomRoomAnyType) :!label _label_2)
                ;;[1 1 1] Sets and checks the length of the Solution Path
                (Math|Integer|IncrementInt (LocalVariables|GetCurrentLength) :!label _label_3
                  (:%20%20
                    (if (>= (LocalVariables|GetCurrentLength) (Variables|LevelConfiguration|GetLengthOfSolutionPath))
                      ;;[1 1 1] Sets the Last Room
                      (Variables|LocalLevelData|SetFinalRoomGridLocation (LocalVariables|GetCurrentPosition))
                      (Utilities|Map|Add (LocalVariables|GetPathMap) (LocalVariables|GetCurrentPosition) (LocalVariables|GetSelectedRoomType))
                      ;;;[1 1 1] Stop Level Generation if completed Required Length
                      (LocalVariables|SetisGenerating false)
                      (else
                        ;;[1 1 1] Sets the First Room
                        (if (== (LocalVariables|GetCurrentLength) 1)
                          (Variables|LocalLevelData|SetStartRoomGridLocation (LocalVariables|GetCurrentPosition))
                          (Utilities|Map|Add (LocalVariables|GetPathMap) (LocalVariables|GetCurrentPosition) "NewEnumerator4")
                          (else
                            ;;[1 1 1] Sets the Middle Room
                            (if (== (LocalVariables|GetCurrentLength) (/ (Variables|LevelConfiguration|GetLengthOfSolutionPath) 2))
                              (Variables|LocalLevelData|SetMiddleRoomGridLocation (LocalVariables|GetCurrentPosition))
                              (Utilities|Map|Add (LocalVariables|GetPathMap) (LocalVariables|GetCurrentPosition) "NewEnumerator4")
                              (else
                                ;;[1 1 1] Sets the Special Room
                                (if (== (LocalVariables|GetCurrentLength) (/ (Variables|LevelConfiguration|GetLengthOfSolutionPath) 2))
                                  (Variables|LocalLevelData|SetSpecialRoomGridLocation (LocalVariables|GetCurrentPosition))
                                  (Utilities|Map|Add (LocalVariables|GetPathMap) (LocalVariables|GetCurrentPosition) "NewEnumerator4")
                                  (else
                                    ;;[1 1 1] Sets All Other Rooms
                                    (Utilities|Map|Add (LocalVariables|GetPathMap) (LocalVariables|GetCurrentPosition) (LocalVariables|GetSelectedRoomType)))))))))))))))
          (:2
            (goto _label))
          (:3
            ;;[1 1 1] Move Left
            (bind _result_2 (Math|Integer|DecrementInt (Utilities|Struct|BreakIntVector (LocalVariables|GetCurrentPosition)) :!label _label_4)
              (:%20%20
                (Utilities|Struct|SetmembersinIntVector (LocalVariables|GetCurrentPosition) _result_2)
                ;;[1 1 1] Next Direction, Can not backtrack
                (LocalVariables|SetDirection (Math|Random|RandomIntegerinRange 3 5))
                (goto _label_2))))
          (:4
            (goto _label_4))
          (:5
            (Math|Integer|IncrementInt (LocalVariables|GetupCounter)
              (:%20%20
                ;;[1 1 1] Does current room have TOP Exit before we move up
                (if (.ReturnValue (Utilities|Map|Find (LocalVariables|GetPathMap) (LocalVariables|GetCurrentPosition)))
                  (switch Utilities|FlowControl|Switch|SwitchonRoomTypes (.Value (Utilities|Map|Find (LocalVariables|GetPathMap) (LocalVariables|GetCurrentPosition)))
                    (:NewEnumerator1
                      ;;[1 1 1] We must change current room to a room with TOP exit
                      (if (>= (LocalVariables|GetupCounter) 2) :!label _label_5
                        (LocalVariables|SetupCounter 0)
                        (Utilities|Map|Add _pathmap (LocalVariables|GetCurrentPosition) "NewEnumerator4")
                        (else
                          (Utilities|Map|Add _pathmap (LocalVariables|GetCurrentPosition) (Utilities|GetRandomRoomwithTopExit)))))
                    (:NewEnumerator2
                      _)
                    (:NewEnumerator4
                      _)
                    (:NewEnumerator0
                      (goto _label_5))
                    (:NewEnumerator7
                      (goto _label_5)))
                  ;;[1 1 1] Move Up
                  (bind _result_3 (Math|Integer|IncrementInt (Utilities|Struct|BreakIntVector (LocalVariables|GetCurrentPosition)))
                    (:%20%20
                      (Utilities|Struct|SetmembersinIntVector (LocalVariables|GetCurrentPosition) _result_3)
                      ;;[1 1 1] Next Direction
                      (LocalVariables|SetDirection (Math|Random|RandomIntegerinRange 1 5))
                      ;;[1 1 1] Add Room With Bottom Exit
                      (LocalVariables|SetSelectedRoomType (Utilities|GetRandomRoomwithBottomExit))
                      (goto _label_3)))
                  (else
                    (LocalVariables|SetisGenerating false))))))))
      ;[0.02628 1 0.09996 1 30] COMPLETE LOOP
      (return (LocalVariables|GetPathMap)))))

(fn SpawnFinalRoomTarget
  (params (CameraLocation :type Vector) (Location :type Vector))
  (bind _returnvalue (Game|SpawnActorfromClass "/Game/TheSpellplanes/Blueprints/Actors/PathMarker.PathMarker_C" (Math|Conversions|ToTransform(Vector) Location) "AlwaysSpawn" 0 0))
  (Default|CustomCulling (Variables|Default|GetSpellplanesInstance) (Variables|/Script/Engine.Actor|GetRootComponent _returnvalue) Location CameraLocation Location false))

(fn PlacePlayerSpawn
  (params (_Location :type Vector))
  (LocalVariables|SetNewPortalLocation _Location)
  (if (Utilities|IsValid (Variables|LocalLevelData|GetCurrentPlayerPortal))
    (Transformation|SetActorLocation (Variables|LocalLevelData|GetCurrentPlayerPortal) (LocalVariables|GetNewPortalLocation) false false)
    (else
      (bind _returnvalue (Game|SpawnActorfromClass "/Game/TheSpellplanes/Blueprints/Actors/BP_PlayerPortal.BP_PlayerPortal_C" (Math|Conversions|ToTransform(Vector) (LocalVariables|GetNewPortalLocation)) "AlwaysSpawn" 0 0))
      (Variables|LocalLevelData|SetCurrentPlayerPortal _returnvalue)
      (bind _asbp_game_instance (Utilities|Casting|CastToBP_GameInstance (Game|GetGameInstance)))
      (bind _roomcenterlocation (Default|GetRoomCenterfromLocation _asbp_game_instance (LocalVariables|GetNewPortalLocation)))
      (Variables|/Game/TheSpellplanes/Blueprints/Actors/BP_PlayerPortal.BP_PlayerPortal_C|SetRoomLocation (Variables|LocalLevelData|GetCurrentPlayerPortal) _roomcenterlocation))))
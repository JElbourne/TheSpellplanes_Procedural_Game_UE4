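; BP_Container is a container block actor that gives the player an inventory to open by interacting with it.
; On BeginPlay it copies its Items array slot by slot into its BPInventoryComponent.
; Interaction from a MySpellPlanesCharacter toggles that component's inventory, and the character leaving the Sphere overlap hides it.
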(event OnComponentEndOverlap(Sphere)
  (params (OverlappedComponent :type Primitive%20Component%20Object%20Reference) (OtherActor :type Actor%20Object%20Reference) (OtherComp :type Primitive%20Component%20Object%20Reference) (OtherBodyIndex :type Integer))
  (Utilities|Casting|CastToMySpellPlanesCharacter OtherActor)
  (CallFunction|HideInventory (Variables|Default|GetBP_InventoryComponent)))

(event Custom|Interact_1
  (params (Interacter :type Character%20Object%20Reference))
  (Utilities|Casting|CastToMySpellPlanesCharacter Interacter)
  (CallFunction|ToggleInventory (Variables|Default|GetBP_InventoryComponent)))

(event EventBeginPlay
  (|CallParentFunction)
  (for (_array_element _array_index) (Variables|Default|Getitems)
    (Utilities|Array|SetArrayElem (Variables|Default|GetInventory (Variables|Default|GetBP_InventoryComponent)) _array_index _array_element)))

(fn ConstructionScript
  (|CallParentFunction))
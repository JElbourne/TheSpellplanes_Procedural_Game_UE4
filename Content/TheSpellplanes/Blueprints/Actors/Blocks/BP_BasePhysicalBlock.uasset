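; BP_BasePhysicalBlock is a damageable block that only takes damage from weapons at or above its required level.
; Health starts full, and each non-lethal hit sets a timer calling "ResetFullHealth", a name this file does not define (its wrapper is CallRestoreFullHealth).
; At zero health it spawns a BP_GridBlock in its place, then destroys itself if the GameInstance removes it from level data.
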(event EventBeginPlay
  (|CallParentFunction)
  (CallFunction|CallRestoreFullHealth))

(event EventTakeDamage
  (params (WeaponLevel :type Integer) (Damage :type Float%20%28single-precision%29))
  (if (>= WeaponLevel (Variables|Default|GetRequiredWeaponLevel))
    (Variables|Default|SetCurrentHealth (- (Variables|Default|GetCurrentHealth) Damage))
    (if (<= (Variables|Default|GetCurrentHealth) 0.0)
      (Utilities|DestroyandReplaceBlock)
      (else
        (Utilities|Time|SetTimerbyFunctionName self "ResetFullHealth" (Variables|Default|GetFullHealthTimer))))))

(fn ConstructionScript
  (|CallParentFunction))

(fn CallRestoreFullHealth
  ;[1 1 1] This is needed so we can call the interface function from the timer.
  (CallFunction|RestoreFullHeath))

(fn RestoreFullHeath
  (Variables|Default|SetCurrentHealth (Variables|Default|GetMaxHealth))
  (return false))
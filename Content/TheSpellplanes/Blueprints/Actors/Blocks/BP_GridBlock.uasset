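; BP_GridBlock is a grid-placed level block actor that registers itself with the game and culls itself as the player moves between rooms.
; On BeginPlay it caches BP_GameInstance, records its location and class in the level data, and subscribes to the walked-into-new-room event.
; On each room change it passes its location, room and the new room center to the GameInstance's shared CustomCulling, with actor destruction enabled.
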(event Custom|BeginBlockCulling
  (params (NewRoomCenterWorldLocation :type Vector))
  (Default|CustomCulling (Variables|Default|GetGameInstance) (Variables|Transformation|GetRootComponent) (Transformation|GetActorLocation) NewRoomCenterWorldLocation (Variables|Default|GetRoomLocation) true))

(event EventBeginPlay
  (bind _asbp_game_instance (Utilities|Casting|CastToBP_GameInstance (Game|GetGameInstance)))
  (bind _output_get (Variables|Default|SetGameInstance _asbp_game_instance))
  (EventDispatchers|BindEventtoWalkedIntoNewRoom _output_get (delegate Custom|BeginBlockCulling))
  (Default|SetBlockinLevelData (Variables|Default|GetGameInstance) (Transformation|GetActorLocation) (Utilities|GetClass self)))

(fn ConstructionScript)
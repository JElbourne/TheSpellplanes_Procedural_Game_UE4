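; Buildings system component that opens and closes the building window UI.
; ToggleWindowUI removes and clears the window if one exists, otherwise creates it and hands it a reference to this component.
; The new widget is added to the first player controller's HUD canvas with anchors spanning the full canvas, rather than directly to the viewport.
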(event EventBeginPlay)

(event EventTick
  (params (DeltaSeconds :type Float%20%28single-precision%29)))

(fn ToggleWindowUI
  (bind _buildingwindowui (Variables|Default|GetBuildingWindowUI)
    (:then
      (Widget|RemovefromParent _buildingwindowui)
      (Variables|Default|SetBuildingWindowUI 0))
    (:else
      (bind _returnvalue (UserInterface|CreateWidget "/Game/TheSpellplanes/Blueprints/BuildingsSystem/UI/BuildingWindowUI.BuildingWindowUI_C"))
      (bind _output_get (Variables|Default|SetBuildingWindowUI _returnvalue))
      (Variables|/Game/TheSpellplanes/Blueprints/BuildingsSystem/UI/BuildingWindowUI.BuildingWindowUI_C|SetBuildingsComponent _output_get self)
      (bind _asplayer_controller (Utilities|Casting|CastToPlayerController (Game|GetPlayerController 0)))
      (bind _returnvalue_2 (Class|CanvasPanel|AddChildtoCanvas (Variables|/Game/TheSpellplanes/UserInterface/GameWidget.GameWidget_C|GetHUDCanvas (Variables|/Game/TheSpellplanes/Blueprints/Controllers/PlayerController.PlayerController_C|GetHudWidget _asplayer_controller)) (Variables|Default|GetBuildingWindowUI)))
      (Class|CanvasPanelSlot|SetAnchors _returnvalue_2 (Utilities|Struct|MakeAnchors "(X=0.000000,Y=0.000000)" "(X=1.000000,Y=1.000000)")))))